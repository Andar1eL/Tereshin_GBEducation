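; Base weapon actor that fires projectiles and tracks its ammunition.
; When Fire is triggered with ActivateGun true, the AmmoAC component checks for and deducts one round, then a BP_AmmoBase spawns at the Arrow component's transform.
; Without ammo it plays a click sound at the weapon's location.
; After either outcome, the Ammo text is refreshed to show current and maximum counts.
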(event Custom|Fire
  (params (ActivateGun :type Boolean))
  (bind _ammoac (Variables|Default|GetAmmoAC))
  (if ActivateGun
    (Utilities|FlowControl|Sequence
      (:then_0
        (if (Default|CheckAmmo _ammoac 1)
          (Default|SubstructAmmo _ammoac 1)
          ;[1 1 1] Создание снарядов
          (Game|SpawnActorfromClass "/Game/Andrey/Weapon/BP_AmmoBase.BP_AmmoBase_C" (Transformation|GetWorldTransform (Variables|Default|GetArrow)) "AlwaysSpawn" 0 0)
          (else
            (Audio|SpawnSoundatLocation "/Engine/VREditor/Sounds/UI/Click_on_Button.Click_on_Button" (Transformation|GetActorLocation) "0, 0, 0" 1.0 1.0 0.0 0 0))))
      (:then_1
        (Rendering|Components|TextRender|SetText (Variables|Default|GetAmmo) (Utilities|Text|FormatText "{Current}/{Max}" (Variables|/Game/Andrey/Weapon/Ammo_AC.Ammo_AC_C|GetCurrentAmmo (Variables|Default|GetAmmoAC)) (Variables|/Game/Andrey/Weapon/Ammo_AC.Ammo_AC_C|GetMaxAmmo (Variables|Default|GetAmmoAC))))))))

(event Collision|EventActorBeginOverlap
  (params (OtherActor :type Actor%20Object%20Reference)))

(event EventTick
  (params (DeltaSeconds :type Float%20%28single-precision%29)))

(fn ConstructionScript)