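; BP_LaserGun is a continuous-beam weapon that overrides the base Fire event to switch the laser on and off.
; While active, each Tick runs an object-type line trace forward from its Arrow component.
; On a hit it moves the particle effect to the impact point and applies Damage scaled by delta time; otherwise the effect is deactivated.
; The beam trace is drawn only through one-frame debug lines.
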(event EventBeginPlay)

(event Collision|EventActorBeginOverlap
  (params (OtherActor :type Actor%20Object%20Reference)))

(event EventTick
  (params (DeltaSeconds :type Float%20%28single-precision%29))
  (bind _arrow (Variables|Default|GetArrow))
  (bind _returnvalue (Transformation|GetWorldLocation _arrow))
  (if (Variables|Default|GetLaserActive)
    ;[1 1 1] Трейсим перед собой данный с чем столкнулись
    (bind (_outhit _returnvalue_2) (Collision|LineTraceForObjects _returnvalue (+ _returnvalue (* (Math|Vector|GetForwardVector _arrow) 10000)) (Utilities|Array|MakeArray "ObjectTypeQuery2" "ObjectTypeQuery4" "ObjectTypeQuery1" "ObjectTypeQuery3") false 0 "ForOneFrame"))
    (if _returnvalue_2
      ;[0.3322 1 0.2586] Активируем эффект
      (Components|Activation|Activate (Variables|Default|GetParticleSystem) false)
      ;[1 1 1] Изменяем координаты искр, в зависимомти от попадания trace
      (Transformation|SetWorldLocation (Variables|Default|GetParticleSystem) (.Location (Collision|BreakHitResult _outhit)) false false)
      ;[1 1 1] Применяем урон к объекту
      (Game|Damage|ApplyDamage (.HitActor (Collision|BreakHitResult _outhit)) (* (Variables|Default|GetDamage) (Utilities|Time|GetWorldDeltaSeconds)) 0 self)
      (else
        ;[1 0.3342 0.1435] Деактивируем эффект
        (Components|Activation|Deactivate (Variables|Default|GetParticleSystem))))
    (else
      ;[1 1 1] Деактивируем эффект
      (Components|Activation|Deactivate (Variables|Default|GetParticleSystem)))))

(event EventFire
  (params (ActivateGun :type Boolean))
  ;[1 1 1] Перегрузка базовой функции
  (Variables|Default|SetLaserActive ActivateGun))

(fn ConstructionScript
  (|CallParentFunction))