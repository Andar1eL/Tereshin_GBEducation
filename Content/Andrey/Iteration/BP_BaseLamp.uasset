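; BP_BaseLamp is an interactable lamp that turns its point light on or off.
; Its overridden ActivateInteract event stores the incoming state and passes it to SwitchLight.
; SwitchLight toggles the PointLight by setting its intensity to a fixed bright value or zero, rather than changing visibility.
; The construction script and TestFunction are empty.
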(event EventActivateInteract
  (params (ActivateInteract :type Boolean))
  ;[1 1 1] Перегруженное событие активации
  (bind _output_get (Variables|Default|SetOnActive ActivateInteract))
  (Variables|Default|Seton/off _output_get)
  (CallFunction|SwitchLight (Variables|Default|Geton/off)))

(fn ConstructionScript)

(fn SwitchLight
  (params (on/off :type Boolean))
  (Variables|Default|Seton/off on/off)
  (if (Variables|Default|Geton/off)
    (Rendering|Components|Light|SetIntensity (Variables|Default|GetPointLight) 5e+03)
    (else
      (Rendering|Components|Light|SetIntensity (Variables|Default|GetPointLight) 0.0))))

(fn TestFunction)