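; Hover platform actor that uses physics forces to float its Platform component above surfaces below it.
; Each Tick it line-traces straight down for world static and dynamic objects, drawing the trace for debugging.
; On a hit it applies an upward, mass-independent force that grows linearly as the surface gets closer, acting like a spring without explicit damping.
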(event EventBeginPlay)

(event Collision|EventActorBeginOverlap
  (params (OtherActor :type Actor%20Object%20Reference)))

(event EventTick
  (params (DeltaSeconds :type Float%20%28single-precision%29))
  ;[0.6968 1 0.3538] Может выдавать как результат столкновения или другие данные
  ;;[0.04174 0.3021 0] LineTrace линия меж двумя точкаии в пространстве
  (bind (_outhit _returnvalue) (Collision|LineTraceForObjects (Transformation|GetWorldLocation (Variables|Default|GetPlatform)) (+ (Transformation|GetWorldLocation (Variables|Default|GetPlatform)) "0, 0,-750.000000") (Utilities|Array|MakeArray "ObjectTypeQuery2" "ObjectTypeQuery1") false 0 "ForOneFrame"))
  (if _returnvalue
    ;[0.3395 0.427 1] Применяем силу в указанном направлении к объекту
    (Physics|AddForce (Variables|Default|GetPlatform) (* "0, 0,5000.000000" (- 1.0 (.Time (Collision|BreakHitResult _outhit)))) "None" true)))

(fn ConstructionScript)