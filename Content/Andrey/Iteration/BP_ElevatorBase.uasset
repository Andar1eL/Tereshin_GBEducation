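; BP_ElevatorBase is an interactable elevator that moves its static mesh along a spline.
; ActivateInteract calls the parent, then plays the MovingScale timeline when OnActive is true or reverses it otherwise.
; Each timeline update samples the spline by time in world space, setting the mesh location and applying only the spline's yaw so it stays level.
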(event EventActivateInteract
  (params (ActivateInteract :type Boolean))
  (|CallParentFunction ActivateInteract)
  (if (Variables|Default|GetOnActive)
    (bind _movingscale (Timeline|MovingScale Play)
      (:Update
        (Transformation|SetWorldLocation (Variables|Default|GetStaticMesh) (Spline|GetLocationatTime (Variables|Default|GetSpline) _movingscale "World" false) false false)
        (Transformation|SetWorldRotation (Variables|Default|GetStaticMesh) (Math|Rotator|MakeRotator 0.0 0.0 (.Yaw (Math|Rotator|BreakRotator (Class|SplineComponent|GetRotationatTime (Variables|Default|GetSpline) _movingscale "World" false)))) false false)))
    (else
      (Timeline|MovingScale Reverse))))

(fn ConstructionScript
  (|CallParentFunction))